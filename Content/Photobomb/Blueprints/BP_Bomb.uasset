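; BP_Bomb is a timed bomb actor for the Photobomb game that explodes ten seconds after BeginPlay.
; Explode briefly scales up its sphere collision as the blast area, activates the particle system and plays the explosion audio event at the bomb mesh's location.
; After a short delay it restores the sphere's scale and destroys itself.
; The file holds no overlap or damage logic.
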(event Custom|Explode
  (Transformation|SetWorldScale3D (Variables|Default|GetSphereCol) "15.000000,15.000000,15.000000")
  (Components|Activation|Activate (Variables|Default|GetParticleSystem) false)
  (Class|FMODBlueprintStatics|PlayEventatLocation "/Game/FMOD/Events/Explosion.Explosion" (Math|Conversions|ToTransform(Vector) (Transformation|GetWorldLocation (Variables|Default|GetBomb))))
  (Utilities|FlowControl|Delay 0.3)
  (Transformation|SetWorldScale3D (Variables|Default|GetSphereCol) "1.000000,1.000000,1.000000")
  (Actor|DestroyActor))

(event EventBeginPlay
  (Utilities|FlowControl|Delay 1e+01)
  (CallFunction|Explode))

(fn ConstructionScript)